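; BP_Quadcopter is a quadcopter that holds and adjusts its altitude using four engine components.
; Each tick, throttle input shifts a desired altitude that starts at the spawn height.
; A PID calculation compares it with actual height, and the negated, scaled result is applied as the same upward force on every engine.
; Roll, pitch and attitude stabilization are empty stubs that never run.
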(event `self.ReceiveBeginPlay`
  (bind (_returnvalue_x _returnvalue_y _returnvalue_z) (`KismetMathLibrary.BreakVector` (`self.K2_GetActorLocation`)))
  (set `self.DesiredAltitude` _returnvalue_z))

(event `self.ReceiveTick`
  (params (DeltaSeconds :type "Float (single-precision)"))
  (`self.Handle Throttle` DeltaSeconds)
  (`self.AltitudeStabilization` DeltaSeconds))

(fn `AltitudeStabilization`
  (params (`Delta Time` :type "Float (double-precision)"))
  (bind (_returnvalue_x _returnvalue_y _returnvalue_z) (`KismetMathLibrary.BreakVector` (`self.K2_GetActorLocation`)))
  (bind _value (`/Game/Fly/BPF_PID.PDICalculations` _returnvalue_z (`self.DesiredAltitude`) 0.2 0.005 0.1 (`self.AltitudeStabilizationForceMultiplier`) `Delta Time` (`self.AltitudeControlIntegral`) (`self.AltitudeControlErrorPrior`)))
  (for _array_element (`self.EngineArray`)
    (`/Game/Fly/EngineComponent.AddUPForce` _array_element (* (* _value -1.0) (`self.AltitudeStabilizationForceMultiplier`))))
  (return))

(fn `Handle Throttle`
  (params (`Delta Time` :type "Float (double-precision)"))
  (set `self.DesiredAltitude` (+ (`self.DesiredAltitude`) (* (* `Delta Time` (`self.GetInputAxisValue`)) (`self.ManualThrottleForceMultiplier`)))))

(fn `HandlePitch`
  (params (`Delta Time` :type "Float (double-precision)")))

(fn `HandleRoll`
  (params (`Delta Time` :type "Float (double-precision)")))

(fn `Stabilize`
  (params (`Delta Time` :type "Float (double-precision)")))

(fn `UserConstructionScript`
  (set `self.EngineArray` (`|MakeArray` (`self.Engine1`) (`self.Engine2`) (`self.Engine3`) (`self.Engine4`))))